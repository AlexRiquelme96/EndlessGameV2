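; BP_Unit is a unit Blueprint whose skeletal mesh and animation change with its UnitType: MainWarrior, Ranger, Warrior or Slime.
; The construction script selects the matching mesh asset and Animation Blueprint.
; From BeginPlay, an endless delay loop advances a test index through five animation states every three seconds and sends each to the AnimInstance as a message, cycling the animations for testing.
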(event `self.ReceiveBeginPlay`
  (`KismetSystemLibrary.Delay` 3.0 :!label _label)
  (bind _output_get (set `self.TestAnimIndex` (cast `/Game/Art/Units/E_UnitAnimationStates` (mod (+ (`self.TestAnimIndex`) 1) 5))))
  (message `/Game/Art/Units/BPI_UnitAnimation.SetUnitAnimationState` (`SkeletalMeshComponent.GetAnimInstance` (`self.SkeletalMesh`)) _output_get)
  (goto _label))

(fn `UserConstructionScript`
  (bind _skeletalmesh (`self.SkeletalMesh`))
  (`SkeletalMeshComponent.SetSkeletalMeshAsset` _skeletalmesh (select `/Game/Art/Units/E_UnitType` (`self.UnitType`) :`NewEnumerator0` "/Game/Art/Units/Main_Warrior/Main_Warrior.Main_Warrior" :`NewEnumerator1` "/Game/Art/Units/Ranger/SK_Ranger.SK_Ranger" :`NewEnumerator2` "/Game/Art/Units/Warrior/SK_Warrior.SK_Warrior" :`NewEnumerator3` "/Game/Art/Units/Slime/Slime.Slime" :!type "SkeletalMesh Object Reference"))
  (`SkeletalMeshComponent.SetAnimInstanceClass` _skeletalmesh (select `/Game/Art/Units/E_UnitType` (`self.UnitType`) :`NewEnumerator0` "/Game/Art/Units/Main_Warrior/ABP_Main_Warrior.ABP_Main_Warrior_C" :`NewEnumerator1` "/Game/Art/Units/Ranger/ABP_Ranger.ABP_Ranger_C" :`NewEnumerator2` "/Game/Art/Units/Warrior/ABP_Warrior.ABP_Warrior_C" :`NewEnumerator3` "/Game/Art/Units/Slime/ABP_Slime.ABP_Slime_C" :!type "Object Class Reference")))