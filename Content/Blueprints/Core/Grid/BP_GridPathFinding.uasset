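; Grid pathfinding Blueprint that runs A* over square or hexagon tiles, filtering neighbors by tile type and height difference.
; A cost-sorted discovered list weighs entry costs plus a distance heuristic, favoring non-diagonal steps on ties.
; Search stops when the target is first discovered, then rebuilds the path from previous-tile links.
; FindPath runs synchronously or, given a delay, time-sliced by a millisecond budget, reporting through callbacks.
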(event `FindPathWithDelay`
  (`|ExecutionSequence`
    (:`then_0`
      (goto _label_3 :!via `Open`))
    (:`then_1`
      (set `self.LoopStartTime` (`KismetMathLibrary.Now`) :!label _label)
      (if (> (`KismetArrayLibrary.Array_Length` (`self.DiscoveredTileIndexes`)) 0) :!label _label_2
        (bind _foundtargettile (`self.AnalyseNextDiscoveredTile`))
        (if _foundtargettile
          (bind _path (`self.GeneratePath`))
          (`self.OnPathFindingCompleted` _path)
          (else
            (if (> (`self.MaxMsPerFrame`) 0.0)
              (if (< (`KismetMathLibrary.GetTotalMilliseconds` (- (`KismetMathLibrary.Now`) (`self.LoopStartTime`))) (`self.MaxMsPerFrame`))
                (goto _label_2)
                (else
                  _)))
            (`KismetSystemLibrary.RetriggerableDelay` (`self.DelayBetweenIterations`))
            (`/Engine/EditorBlueprintResources/StandardMacros.Gate` true :!label _label_3
              (:`Exit`
                (goto _label)))))
        (else
          (`self.OnPathFindingCompleted` (`|MakeArray`)))))))

(event `CloseDelayGate`
  (goto _label_3 :!via `Close`))

(fn `AnalyseNextDiscoveredTile`
  (returns (FoundTargetTile :type Boolean))
  (bind _tilepathdata (`self.PullCheapestTileOutOfDiscoveredList`))
  (bind _output_get (set `self.CurrentDiscoveredTile` _tilepathdata))
  (`self.OnPathFindingDataUpdated` (`.Index_2_80A1FE8D45E6BF2D728E52B5CA1D7299` (break `/Game/Blueprints/Core/Grid/Utilities/S_PathFindingData` _output_get)))
  (bind _neighbors (`self.GetValidTileNeighbors` (`.Index_2_80A1FE8D45E6BF2D728E52B5CA1D7299` (break `/Game/Blueprints/Core/Grid/Utilities/S_PathFindingData` (`self.CurrentDiscoveredTile`))) (`self.Include Diagonals`) (`self.ValidTileTypes`)))
  (set `self.CurrentNeighbors` _neighbors)
  (while (> (`KismetArrayLibrary.Array_Length` (`self.CurrentNeighbors`)) 0)
    (bind _istargettile (`self.DiscoverNextNeighbor`))
    (if _istargettile
      (return true)))
  (return false))

(fn `ClearGeneratedData`
  (`BlueprintMapLibrary.Map_Clear` (`self.PathFindingData`))
  (`KismetArrayLibrary.Array_Clear` (`self.DiscoveredTileSortingCost`))
  (`KismetArrayLibrary.Array_Clear` (`self.DiscoveredTileIndexes`))
  (`KismetArrayLibrary.Array_Clear` (`self.AnalysedTileIndexes`))
  (`self.OnPathFindingDataCleared`))

(fn `DiscoverNextNeighbor`
  (returns (IsTargetTile :type Boolean))
  (locals (CostFromStart :type Integer) (IndexDiscovered :type Integer :default 0))
  (bind _indexdiscovered (`local.IndexDiscovered`))
  (bind (_index _costtoentertile) (break `/Game/Blueprints/Core/Grid/Utilities/S_PathFindingData` (`self.CurrentNeighbor`)))
  (set `self.CurrentNeighbor` (`|GetArrayItem` (`self.CurrentNeighbors`)))
  (`KismetArrayLibrary.Array_Remove` (`self.CurrentNeighbors`))
  (if (not (`KismetArrayLibrary.Array_Contains` (`self.AnalysedTileIndexes`) (`.Index_2_80A1FE8D45E6BF2D728E52B5CA1D7299` (break `/Game/Blueprints/Core/Grid/Utilities/S_PathFindingData` (`self.CurrentNeighbor`)))))
    (set `local.CostFromStart` (+ (`.CostFromStart_9_8EFD7D584741B82BDE745DB7B429C0CB` (break `/Game/Blueprints/Core/Grid/Utilities/S_PathFindingData` (`self.CurrentDiscoveredTile`))) (`.CostToEnterTile_7_7DB4A3EB4D7F34D8071B49BA5ADD9E4D` (break `/Game/Blueprints/Core/Grid/Utilities/S_PathFindingData` (`self.CurrentNeighbor`)))))
    (bind _output_get (set `local.IndexDiscovered` (`KismetArrayLibrary.Array_Find` (`self.DiscoveredTileIndexes`) (`.Index_2_80A1FE8D45E6BF2D728E52B5CA1D7299` (break `/Game/Blueprints/Core/Grid/Utilities/S_PathFindingData` (`self.CurrentNeighbor`))))))
    (if (not (== _output_get -1))
      (bind _output_get_2 (set `self.CurrentNeighbor` (`BlueprintMapLibrary.Map_Find` (`self.PathFindingData`) (`.Index_2_80A1FE8D45E6BF2D728E52B5CA1D7299` (break `/Game/Blueprints/Core/Grid/Utilities/S_PathFindingData` (`self.CurrentNeighbor`))))))
      (if (< (`local.CostFromStart`) (`.CostFromStart_9_8EFD7D584741B82BDE745DB7B429C0CB` (break `/Game/Blueprints/Core/Grid/Utilities/S_PathFindingData` _output_get_2)))
        (`KismetArrayLibrary.Array_Remove` (`self.DiscoveredTileIndexes`) _indexdiscovered)
        (`KismetArrayLibrary.Array_Remove` (`self.DiscoveredTileSortingCost`) _indexdiscovered)
        (else
          (return false))))
    (`self.DiscoverTile` (make `/Game/Blueprints/Core/Grid/Utilities/S_PathFindingData` _index _costtoentertile (`local.CostFromStart`) (`self.GetMinimumCostBetweenTwoTiles` (`.Index_2_80A1FE8D45E6BF2D728E52B5CA1D7299` (break `/Game/Blueprints/Core/Grid/Utilities/S_PathFindingData` (`self.CurrentNeighbor`))) (`self.Target Index`) (`self.Include Diagonals`)) (`.Index_2_80A1FE8D45E6BF2D728E52B5CA1D7299` (break `/Game/Blueprints/Core/Grid/Utilities/S_PathFindingData` (`self.CurrentDiscoveredTile`)))))
    (if (`KismetMathLibrary.Equal_IntPointIntPoint` (`.Index_2_80A1FE8D45E6BF2D728E52B5CA1D7299` (break `/Game/Blueprints/Core/Grid/Utilities/S_PathFindingData` (`self.CurrentNeighbor`))) (`self.Target Index`))
      (return true)
      (else
        (return false)))
    (else
      (return false))))

(fn `DiscoverTile`
  (params (TilePathData :type "/Game/Blueprints/Core/Grid/Utilities/S_PathFindingData Structure"))
  (bind _index (break `/Game/Blueprints/Core/Grid/Utilities/S_PathFindingData` TilePathData))
  (`BlueprintMapLibrary.Map_Add` (`self.PathFindingData`) _index TilePathData)
  (`self.InsertTileInDiscoveredArray` TilePathData)
  (`self.OnPathFindingDataUpdated` _index))

(fn `FindPath`
  (params (Start :type "IntPoint Structure") (Target :type "IntPoint Structure") (Diagonals :type Boolean) (TileTypes :type "Array of /Game/Blueprints/Core/Grid/Utilities/E_TileType Enum") (Delay :type "Float (double-precision)") (MaxMs :type "Float (double-precision)"))
  (returns (Path :type "Array of IntPoint Structure"))
  (bind _array (`|MakeArray`))
  (bind _array_2 (`|MakeArray`))
  (set `self.Start Index` Start)
  (set `self.Target Index` Target)
  (set `self.Include Diagonals` Diagonals)
  (set `self.ValidTileTypes` TileTypes)
  (set `self.DelayBetweenIterations` Delay)
  (set `self.MaxMsPerFrame` MaxMs)
  (`self.CloseDelayGate`)
  (`self.ClearGeneratedData`)
  (bind _isvalid (`self.IsInputDataValid`))
  (if _isvalid
    (`self.DiscoverTile` (make `/Game/Blueprints/Core/Grid/Utilities/S_PathFindingData` (`self.Start Index`) 1 0 (`self.GetMinimumCostBetweenTwoTiles` (`self.Start Index`) (`self.Target Index`) (`self.Include Diagonals`))))
    (if (<= (`self.DelayBetweenIterations`) 0.0)
      (while (> (`KismetArrayLibrary.Array_Length` (`self.DiscoveredTileIndexes`)) 0)
        (bind _foundtargettile (`self.AnalyseNextDiscoveredTile`))
        (if _foundtargettile
          (bind _path (`self.GeneratePath`))
          (`self.OnPathFindingCompleted` _path)
          (return _path)))
      (`self.OnPathFindingCompleted` _array)
      (return _array)
      (else
        (`self.FindPathWithDelay`)
        (return (`|MakeArray`))))
    (else
      (`self.OnPathFindingCompleted` _array_2)
      (return _array_2))))

(fn `GeneratePath`
  (returns (Path :type "Array of IntPoint Structure"))
  (locals (Current :type "IntPoint Structure") (InvertedPath :type "Array of IntPoint Structure") (Ret :type "Array of IntPoint Structure"))
  (set `local.Current` (`self.Target Index`))
  (while (!= (`local.Current`) (`self.Start Index`))
    (`KismetArrayLibrary.Array_Add` (`local.InvertedPath`) (`local.Current`))
    (set `local.Current` (`.PreviousIndex_4_3F6668A6441060A14E9A6B9CCAC3A5A6` (break `/Game/Blueprints/Core/Grid/Utilities/S_PathFindingData` (`BlueprintMapLibrary.Map_Find` (`self.PathFindingData`) (`local.Current`))))))
  (bind (_arrayindex _arrayelement) (`/Engine/EditorBlueprintResources/StandardMacros.ReverseForEachLoop` (`local.InvertedPath`))
    (:`LoopBody`
      (`KismetArrayLibrary.Array_Add` (`local.Ret`) _arrayelement))
    (:`Completed`
      (return (`local.Ret`)))))

(fn `GetMinimumCostBetweenTwoTiles`
  (params (Index1 :type "IntPoint Structure") (Index2 :type "IntPoint Structure") (Diagonals :type Boolean))
  (returns (MinCost :type Integer))
  (bind (_returnvalue_x _returnvalue_y) (break `IntPoint` (- (`local.Index1`) (`local.Index2`))))
  (bind (_returnvalue_x_2 _returnvalue_y_2) (break `IntPoint` (- (`local.Index1`) (`local.Index2`))))
  (bind (_returnvalue_x_3 _returnvalue_y_3) (break `IntPoint` (- (`local.Index1`) (`local.Index2`))))
  (bind _returnvalue (`KismetMathLibrary.Abs_Int` _returnvalue_x))
  (switch `/Game/Blueprints/Core/Grid/GridShapes/E_GridShapeData` (`/Game/Blueprints/Core/Grid/BP_Grid.GridShape` (`self.Grid`))
    (:`NewEnumerator1`
      (return (+ _returnvalue (`KismetMathLibrary.Max` (/ (- (`KismetMathLibrary.Abs_Int` _returnvalue_y) _returnvalue) 2)))))
    (:`NewEnumerator3`
      (if (`local.Diagonals`)
        (return (`KismetMathLibrary.Max` (`KismetMathLibrary.Abs_Int` _returnvalue_x_2) (`KismetMathLibrary.Abs_Int` _returnvalue_y_2)))
        (else
          (return (+ (`KismetMathLibrary.Abs_Int` _returnvalue_x_3) (`KismetMathLibrary.Abs_Int` _returnvalue_y_3))))))))

(fn `GetNeighborIndexes`
  (params (Index :type "IntPoint Structure") (IncludeDiagonals :type Boolean))
  (returns (Neighbors :type "Array of IntPoint Structure"))
  (switch `/Game/Blueprints/Core/Grid/GridShapes/E_GridShapeData` (`/Game/Blueprints/Core/Grid/BP_Grid.GridShape` (`self.Grid`))
    (:`NewEnumerator1`
      (return (`self.GetNeighborIndexForHexagon` (`local.Index`))))
    (:`NewEnumerator3`
      (return (`self.GetNeighborIndexesForSquare` (`local.Index`) (`local.IncludeDiagonals`))))))

(fn `GetNeighborIndexesForSquare`
  (params (Index :type "IntPoint Structure") (IncludeDiagonals :type Boolean))
  (returns (Neighbors :type "Array of IntPoint Structure"))
  (locals (Ret :type "Array of IntPoint Structure"))
  (bind _array (`|MakeArray` (+ (`local.Index`) (make `IntPoint` 1)) (+ (`local.Index`) (make `IntPoint` 0 1)) (+ (`local.Index`) (make `IntPoint` -1)) (+ (`local.Index`) (make `IntPoint` 0 -1))))
  (if IncludeDiagonals
    (set `local.Ret` _array)
    (`KismetArrayLibrary.Array_Append` (`local.Ret`) (`|MakeArray` (+ (`local.Index`) (make `IntPoint` 1 1)) (+ (`local.Index`) (make `IntPoint` -1 1)) (+ (`local.Index`) (make `IntPoint` -1 -1)) (+ (`local.Index`) (make `IntPoint` 1 -1))))
    (return (`local.Ret`))
    (else
      (return _array))))

(fn `GetNeighborIndexForHexagon`
  (params (Index :type "IntPoint Structure"))
  (returns (Neighbors :type "Array of IntPoint Structure"))
  (return (`|MakeArray` (+ (`local.Index`) (make `IntPoint` 1 1)) (+ (`local.Index`) (make `IntPoint` 0 2)) (+ (`local.Index`) (make `IntPoint` -1 1)) (+ (`local.Index`) (make `IntPoint` -1 -1)) (+ (`local.Index`) (make `IntPoint` 0 -2)) (+ (`local.Index`) (make `IntPoint` 1 -1)))))

(fn `GetTileSortingCost`
  (params (TileData :type "/Game/Blueprints/Core/Grid/Utilities/S_PathFindingData Structure (by ref)"))
  (returns (Cost :type Integer))
  (bind (_index _costtoentertile _costfromstart _minimumcosttotarget) (break `/Game/Blueprints/Core/Grid/Utilities/S_PathFindingData` TileData))
  (bind (_index_2 _costtoentertile_2 _costfromstart_2 _minimumcosttotarget_2 _previousindex) (break `/Game/Blueprints/Core/Grid/Utilities/S_PathFindingData` TileData))
  (return (+ (* (+ _costfromstart _minimumcosttotarget) 2) (`KismetMathLibrary.Conv_BoolToInt` (`self.IsDiagonal` _index_2 _previousindex)))))

(fn `GetValidTileNeighbors`
  (params (Index :type "IntPoint Structure") (IncludeDiagonals :type Boolean) (ValidTypes :type "Array of /Game/Blueprints/Core/Grid/Utilities/E_TileType Enum"))
  (returns (Neighbors :type "Array of /Game/Blueprints/Core/Grid/Utilities/S_PathFindingData Structure"))
  (locals (Data :type "/Game/Blueprints/Core/Grid/Utilities/S_TileData Structure") (InputData :type "/Game/Blueprints/Core/Grid/Utilities/S_TileData Structure") (Ret :type "Array of /Game/Blueprints/Core/Grid/Utilities/S_PathFindingData Structure"))
  (bind (_data_index _data_type) (break `/Game/Blueprints/Core/Grid/Utilities/S_TileData` (`local.Data`)))
  (bind (_data_index_2 _data_type_2) (break `/Game/Blueprints/Core/Grid/Utilities/S_TileData` (`local.Data`)))
  (set `local.InputData` (`BlueprintMapLibrary.Map_Find` (`/Game/Blueprints/Core/Grid/BP_Grid.GridTiles` (`self.Grid`)) (`local.Index`)))
  (bind _neighbors (`self.GetNeighborIndexes` (`local.Index`) (`local.IncludeDiagonals`)))
  (for _array_element _neighbors
    (set `local.Data` (`BlueprintMapLibrary.Map_Find` (`/Game/Blueprints/Core/Grid/BP_Grid.GridTiles` (`self.Grid`)) _array_element))
    (if (`KismetArrayLibrary.Array_Contains` (`local.ValidTypes`) _data_type_2)
      (if (<= (`KismetMathLibrary.Abs` (- (.z (.location (`.Transform_10_01710C414ABE2F39CF11989D84AB3370` (break `/Game/Blueprints/Core/Grid/Utilities/S_TileData` (`local.Data`))))) (.z (.location (`.Transform_10_01710C414ABE2F39CF11989D84AB3370` (break `/Game/Blueprints/Core/Grid/Utilities/S_TileData` (`local.InputData`))))))) 75.0)
        (`KismetArrayLibrary.Array_Add` (`local.Ret`) (make `/Game/Blueprints/Core/Grid/Utilities/S_PathFindingData` _data_index (select `/Game/Blueprints/Core/Grid/Utilities/E_TileType` _data_type :`NewEnumerator1` 1 :`NewEnumerator3` 2 :`NewEnumerator4` 3 :`NewEnumerator5` 1) 999999 999999 (`local.Index`))))))
  (return (`local.Ret`)))

(fn `InsertTileInDiscoveredArray`
  (params (TileData :type "/Game/Blueprints/Core/Grid/Utilities/S_PathFindingData Structure"))
  (locals (SortingCost :type Integer))
  (bind _discoveredtilesortingcost (`self.DiscoveredTileSortingCost`))
  (set `local.SortingCost` (`self.GetTileSortingCost` TileData))
  (if (== (`KismetArrayLibrary.Array_Length` (`self.DiscoveredTileSortingCost`)) 0)
    (`KismetArrayLibrary.Array_Add` (`self.DiscoveredTileSortingCost`) (`local.SortingCost`) :!label _label)
    (`KismetArrayLibrary.Array_Add` (`self.DiscoveredTileIndexes`) (`.Index_2_80A1FE8D45E6BF2D728E52B5CA1D7299` (break `/Game/Blueprints/Core/Grid/Utilities/S_PathFindingData` (`local.TileData`))))
    (elif (>= (`local.SortingCost`) (`|GetArrayItem` _discoveredtilesortingcost (`KismetArrayLibrary.Array_LastIndex` _discoveredtilesortingcost)))
      (goto _label)
      (else
        (for (_array_element _array_index) (`self.DiscoveredTileSortingCost`)
          (if (>= _array_element (`local.SortingCost`))
            (`KismetArrayLibrary.Array_Insert` (`self.DiscoveredTileSortingCost`) (`local.SortingCost`) _array_index)
            (`KismetArrayLibrary.Array_Insert` (`self.DiscoveredTileIndexes`) (`.Index_2_80A1FE8D45E6BF2D728E52B5CA1D7299` (break `/Game/Blueprints/Core/Grid/Utilities/S_PathFindingData` (`local.TileData`))) _array_index)
            (break)))))))

(fn `IsDiagonal`
  (params (index1 :type "IntPoint Structure") (index2 :type "IntPoint Structure"))
  (returns (IsDiagonal :type Boolean))
  (bind _neighbors (`self.GetNeighborIndexes` index1))
  (return (not (`KismetArrayLibrary.Array_Contains` _neighbors index2))))

(fn `IsInputDataValid`
  (returns (IsValid :type Boolean))
  (if (!= (`self.Start Index`) (`self.Target Index`))
    (if (`/Game/Blueprints/Core/Grid/BP_Grid.IsTileWalkable` (`self.Grid`) (`self.Start Index`))
      (if (`/Game/Blueprints/Core/Grid/BP_Grid.IsTileWalkable` (`self.Grid`) (`self.Target Index`))
        (if (`KismetArrayLibrary.Array_Contains` (`self.ValidTileTypes`) (`.Type_7_F49289E54689E707A72D5091FEBA5771` (break `/Game/Blueprints/Core/Grid/Utilities/S_TileData` (`BlueprintMapLibrary.Map_Find` (`/Game/Blueprints/Core/Grid/BP_Grid.GridTiles` (`self.Grid`)) (`self.Target Index`)))))
          (return true)
          (else
            (return false)))
        (else
          (return false)))
      (else
        (return false)))
    (else
      (return false))))

(fn `PullCheapestTileOutOfDiscoveredList`
  (returns (TilePathData :type "/Game/Blueprints/Core/Grid/Utilities/S_PathFindingData Structure"))
  (locals (TileIndex :type "IntPoint Structure"))
  (set `local.TileIndex` (`|GetArrayItem` (`self.DiscoveredTileIndexes`)))
  (`KismetArrayLibrary.Array_Remove` (`self.DiscoveredTileSortingCost`))
  (`KismetArrayLibrary.Array_Remove` (`self.DiscoveredTileIndexes`))
  (`KismetArrayLibrary.Array_Add` (`self.AnalysedTileIndexes`) (`local.TileIndex`))
  (return (`BlueprintMapLibrary.Map_Find` (`self.PathFindingData`) (`local.TileIndex`))))

(fn `UserConstructionScript`)