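; BP_Grid is a grid actor that builds a square, hexagon or triangle tile field as instanced static mesh instances.
; SpawnGrid clears old instances, applies the shape's mesh and material, snaps the center, then derives each tile's transform from its index.
; With environment use on, sphere traces snap tile height to ground hits, and BP_GridModifier hits set tile type so non-walkable tiles are skipped.
; Nothing in this Blueprint calls SpawnGrid on a live path.
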(fn `CalculateCenterAndBottomLeft`
  (returns (Center :type "Vector Structure") (BottomLeft :type "Vector Structure"))
  (locals (C :type "Vector Structure" :default (0.0 0.0 0.0)))
  (bind (_gridtilecount_x _gridtilecount_y) (break `IntPoint` (`self.GridTileCount`)))
  (switch `/Game/Blueprints/Core/Grid/GridShapes/E_GridShapeData` (`self.GridShape`)
    (:`NewEnumerator1`
      (set `local.C` (`/Game/Blueprints/Core/Utilities/BFL_Utilities.SnapVectorToVector` (`self.GridCenterLocation`) (* (`self.GridTileSize`) (1.5 1.0 0.0))))
      (return (`local.C`) (- (`self.GridCenterLocation`) (`/Game/Blueprints/Core/Utilities/BFL_Utilities.SnapVectorToVector` (* (/ (`self.GridTileCount`) (3.0 2.0)) (`KismetMathLibrary.Conv_VectorToVector2D` (`self.GridTileSize`))) (* (`self.GridTileSize`) (1.5 1.0 0.0))))))
    (:`NewEnumerator2`
      (set `local.C` (`/Game/Blueprints/Core/Utilities/BFL_Utilities.SnapVectorToVector` (`self.GridCenterLocation`) (* (`self.GridTileSize`) (2.0 0.0 0.0))))
      (return (`local.C`) (- (`self.GridCenterLocation`) (`/Game/Blueprints/Core/Utilities/BFL_Utilities.SnapVectorToVector` (* (/ (- (`self.GridTileCount`) (1.0 1.0)) (2.0 4.0)) (`KismetMathLibrary.Conv_VectorToVector2D` (`self.GridTileSize`))) (* (`self.GridTileSize`) (2.0 0.0 0.0))))))
    (:`NewEnumerator3`
      (set `local.C` (`/Game/Blueprints/Core/Utilities/BFL_Utilities.SnapVectorToVector` (`self.GridCenterLocation`) (`self.GridTileSize`)))
      (return (`local.C`) (- (`self.GridCenterLocation`) (* (/ (- (`self.GridTileCount`) (`KismetMathLibrary.MakeVector2D` (`KismetMathLibrary.SelectFloat` 0.0 1.0 (`/Game/Blueprints/Core/Utilities/BFL_Utilities.IsIntEven` _gridtilecount_x)) (`KismetMathLibrary.SelectFloat` 0.0 1.0 (`/Game/Blueprints/Core/Utilities/BFL_Utilities.IsIntEven` _gridtilecount_y)))) 2.0) (`KismetMathLibrary.Conv_VectorToVector2D` (`self.GridTileSize`))))))))

(fn `DestroyGrid`
  (`InstancedStaticMeshComponent.ClearInstances` (`self.InstancedStaticMesh`)))

(fn `GetCurrentShapeData`
  (returns (ReturnValue :type "/Game/Blueprints/Core/Grid/GridShapes/S_GridShapeData Structure"))
  (return (`/Game/Blueprints/Core/Grid/GridShapes/BFL_GridShape.GetShapeData` (`self.GridShape`))))

(fn `GetTileLocationFromGridIndex`
  (params (GridIndex :type "IntPoint Structure"))
  (returns (TileLocation :type "Vector Structure"))
  (return (+ (`self.GridBottomLeftCornerLocation`) (* (`self.GridTileSize`) (* GridIndex (select `/Game/Blueprints/Core/Grid/GridShapes/E_GridShapeData` (`self.GridShape`) :`NewEnumerator1` (0.75 0.5) :`NewEnumerator2` (1.0 0.5) :!type "Vector2D Structure"))))))

(fn `GetTileRotationForGridIndex`
  (params (GridIndex :type "IntPoint Structure"))
  (returns (TileRotation :type "Rotator Structure"))
  (bind (_gridindex_x _gridindex_y) (break `IntPoint` (`local.GridIndex`)))
  (if (`|EnumEquality` (`self.GridShape`) "NewEnumerator2")
    (return (`KismetMathLibrary.MakeRotator` 0.0 0.0 (+ (`KismetMathLibrary.SelectFloat` 180.0 0.0 (`/Game/Blueprints/Core/Utilities/BFL_Utilities.IsIntEven` _gridindex_x)) (`KismetMathLibrary.SelectFloat` 180.0 0.0 (`/Game/Blueprints/Core/Utilities/BFL_Utilities.IsIntEven` _gridindex_y)))))
    (else
      (return))))

(fn `IsTileTypeWalkable`
  (params (TileType :type "/Game/Blueprints/Core/Grid/Utilities/E_TileType Enum" :default "NewEnumerator0"))
  (returns (IsWalkable :type Boolean))
  (return (not (`KismetArrayLibrary.Array_Contains` (`|MakeArray` "NewEnumerator0" "NewEnumerator2" :!type "/Game/Blueprints/Core/Grid/Utilities/E_TileType Enum") TileType))))

(fn `SetGridOffsetFromGround`
  (params (Offset :type "Float (double-precision)"))
  (set `self.OffsetFromGround` Offset)
  (`SceneComponent.K2_SetWorldLocation` (`self.InstancedStaticMesh`) (`KismetMathLibrary.MakeVector` 0.0 0.0 (`self.OffsetFromGround`)) false false))

(fn `SpawnGrid`
  (params (CenterLocation :type "Vector Structure") (TileSize :type "Vector Structure") (TileCount :type "IntPoint Structure") (Shape :type "/Game/Blueprints/Core/Grid/GridShapes/E_GridShapeData Enum" :default "NewEnumerator0") (UseEnviroment :type Boolean))
  (locals (X :type Integer) (Y :type Integer) (TileTransform :type "Transform Structure") (Index :type "IntPoint Structure"))
  (bind _instancedstaticmesh (`self.InstancedStaticMesh`))
  (bind (_gridtilecount_x _gridtilecount_y) (break `IntPoint` (`self.GridTileCount`)))
  (bind _gridtilecount_x_2 (break `IntPoint` (`self.GridTileCount`)))
  (bind (_tiletransform_location _tiletransform_rotation _tiletransform_scale) (`KismetMathLibrary.BreakTransform` (`local.TileTransform`)))
  (bind (_gridtilecount_x_3 _gridtilecount_y_2) (break `IntPoint` (`self.GridTileCount`)))
  (bind (_meshsize _mesh _meshmaterial _flatmesh _flatbordermaterial) (break `/Game/Blueprints/Core/Grid/GridShapes/S_GridShapeData` (`self.GetCurrentShapeData`)))
  (set `self.GridCenterLocation` CenterLocation)
  (set `self.GridTileSize` TileSize)
  (set `self.GridTileCount` TileCount)
  (set `self.GridShape` Shape)
  (`self.DestroyGrid`)
  (`StaticMeshComponent.SetStaticMesh` _instancedstaticmesh _flatmesh)
  (`PrimitiveComponent.SetMaterial` _instancedstaticmesh 0 _flatbordermaterial)
  (bind (_center _bottomleft) (`self.CalculateCenterAndBottomLeft`))
  (`self.SetGridOffsetFromGround` (`self.OffsetFromGround`))
  (set `self.GridCenterLocation` _center)
  (set `self.GridBottomLeftCornerLocation` _bottomleft)
  (for _index (range _gridtilecount_x_2)
    (set `local.X` _index)
    (if (`|EnumInequality` (`self.GridShape`) "NewEnumerator1")
      (for _index_2 (range _gridtilecount_y_2)
        (set `local.Y` _index_2)
        (set `local.Index` (make `IntPoint` (`local.X`) (`local.Y`)) :!label _label)
        (set `local.TileTransform` (`KismetMathLibrary.MakeTransform` (`self.GetTileLocationFromGridIndex` (`local.Index`)) (`self.GetTileRotationForGridIndex` (`local.Index`)) (/ (`self.GridTileSize`) (`.MeshSize_2_D36F90E44F98513A05EEF2B60D26F5F8` (break `/Game/Blueprints/Core/Grid/GridShapes/S_GridShapeData` (`self.GetCurrentShapeData`))))))
        (if (`local.UseEnviroment`)
          (bind (_tiletype _outlocation) (`self.TraceForGround` _tiletransform_location))
          (if (`self.IsTileTypeWalkable` _tiletype)
            (set `local.TileTransform` (`KismetMathLibrary.MakeTransform` _outlocation _tiletransform_rotation _tiletransform_scale))
            (`InstancedStaticMeshComponent.AddInstance` (`self.InstancedStaticMesh`) (`local.TileTransform`) false))
          (else
            (`InstancedStaticMeshComponent.AddInstance` (`self.InstancedStaticMesh`) (`local.TileTransform`) false))))
      (else
        (for _index_3 (range (`KismetMathLibrary.SelectInt` 0 1 (`/Game/Blueprints/Core/Utilities/BFL_Utilities.IsIntEven` (`local.X`))) (* _gridtilecount_y 2))
          (set `local.Y` _index_3)
          (`|ExecutionSequence`
            (:`then_0`
              (goto _label))
            (:`then_1`
              (`/Engine/EditorBlueprintResources/StandardMacros.IncrementInt` _index_3))))))))

(fn `TraceForGround`
  (params (Location :type "Vector Structure"))
  (returns (TileType :type "/Game/Blueprints/Core/Grid/Utilities/E_TileType Enum") (OutLocation :type "Vector Structure"))
  (locals (RetType :type "/Game/Blueprints/Core/Grid/Utilities/E_TileType Enum" :default "NewEnumerator0") (RetZ :type "Float (double-precision)" :default 0.0))
  (bind _gridtilesize_x (`KismetMathLibrary.BreakVector` (`self.GridTileSize`)))
  (bind _location (`local.Location`))
  (bind (_location_x _location_y) (`KismetMathLibrary.BreakVector` (`local.Location`)))
  (bind (_gridtilesize_x_2 _gridtilesize_y _gridtilesize_z) (`KismetMathLibrary.BreakVector` (`self.GridTileSize`)))
  (set `self.Radius` (/ _gridtilesize_x (`KismetMathLibrary.SelectFloat` 8.0 3.0 (`|EnumEquality` (`self.GridShape`) "NewEnumerator2"))))
  (bind _outhits (`KismetSystemLibrary.SphereTraceMulti` (+ _location (0.0 0.0 100.0)) (+ _location (0.0 0.0 100.0)) (`self.Radius`) "TraceTypeQuery3"))
  (if (> (`KismetArrayLibrary.Array_Length` _outhits) 0)
    (set `local.RetType` "NewEnumerator1")
    (for _array_element _outhits
      (bind (_bblockinghit _binitialoverlap _time _distance _location_2 _impactpoint _normal _impactnormal _physmat _hitactor) (`GameplayStatics.BreakHitResult` _array_element))
      (bind _asbp_grid_modifier (cast `/Game/Blueprints/Core/Grid/BP_GridModifier` _hitactor)
        (:`then`
          (set `local.RetType` (`/Game/Blueprints/Core/Grid/BP_GridModifier.Type` _asbp_grid_modifier)))
        (:`CastFailed`
          (set `local.RetZ` (`KismetMathLibrary.GridSnap_Float` (- (.z _location_2) (`self.Radius`)) _gridtilesize_z)))))
    (return (`local.RetType`) (`KismetMathLibrary.MakeVector` _location_x _location_y (`local.RetZ`)))
    (else
      (return "NewEnumerator0" (`local.Location`)))))

(fn `UserConstructionScript`)